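; BP_PlayerRobo is a player robot Blueprint that sets up Enhanced Input and so far only prints input for debugging.
; On BeginPlay it adds the INC_3rdPerson mapping context to player controller 0's Enhanced Input subsystem.
; Jump, Move and Look actions print their values or a jump message to screen, with no movement or camera logic implemented yet.
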(event `self.ReceiveBeginPlay`
  (bind _returnvalue (pcsubsystem `EnhancedInputLocalPlayerSubsystem` (`GameplayStatics.GetPlayerController` 0)))
  (`/Engine/EditorBlueprintResources/StandardMacros.IsValid` _returnvalue
    (:`Is Valid`
      (`EnhancedInputSubsystemInterface.AddMappingContext` _returnvalue "/Game/INC_3rdPerson.INC_3rdPerson" 0 (struct)))))

(event `EnhancedInput|/Game/INP_Jump`
  (params (ActionValue :type Boolean) (ElapsedSeconds :type "Float (double-precision)") (TriggeredSeconds :type "Float (double-precision)") (InputAction :type "InputAction Object Reference" :default "/Game/INP_Jump.INP_Jump"))
  (:`Triggered`
    (`KismetSystemLibrary.PrintString` "Jump TRUE"))
  (:`Started`
    (`KismetSystemLibrary.PrintString` (`KismetStringLibrary.Conv_BoolToString` ActionValue) :!label _label))
  (:`Completed`
    (goto _label)))

(event `EnhancedInput|/Game/INP_Move`
  (params (ActionValue :type "Vector2D Structure") (ElapsedSeconds :type "Float (double-precision)") (TriggeredSeconds :type "Float (double-precision)") (InputAction :type "InputAction Object Reference" :default "/Game/INP_Move.INP_Move"))
  (:`Triggered`
    (`KismetSystemLibrary.PrintString` (`KismetStringLibrary.Conv_Vector2dToString` ActionValue))))

(event `EnhancedInput|/Game/INP_Look`
  (params (ActionValue :type "Vector2D Structure") (ElapsedSeconds :type "Float (double-precision)") (TriggeredSeconds :type "Float (double-precision)") (InputAction :type "InputAction Object Reference" :default "/Game/INP_Look.INP_Look"))
  (:`Triggered`
    (`KismetSystemLibrary.PrintString` (`KismetStringLibrary.Conv_Vector2dToString` ActionValue))))

(fn `UserConstructionScript`)